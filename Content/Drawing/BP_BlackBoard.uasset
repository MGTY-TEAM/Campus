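; BP_BlackBoard is a blackboard that the player draws on with a chalk texture while holding interact.
; BeginPlay creates a render target, draws the board material into it, feeds it to the mesh's dynamic board material and creates a dynamic brush material.
; HoldInteract re-traces the hit with complex collision and converts it to UV through FindCollisionUV.
; DrawBrush stamps the brush material onto the render target canvas at that UV.
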(event `self.ReceiveBeginPlay`
  (`|ExecutionSequence`
    (:`then_0`
      ;[1 1 1] Creating a drawing area
      (bind _returnvalue (`KismetRenderingLibrary.CreateRenderTarget2D` 512 512))
      (bind _output_get (set `self.RenderTarget` _returnvalue))
      (`KismetRenderingLibrary.ClearRenderTarget2D` _output_get)
      (`KismetRenderingLibrary.DrawMaterialToRenderTarget` _output_get "/Game/Drawing/M_Board.M_Board"))
    (:`then_1`
      ;[1 1 1] Loading the board material
      (bind _returnvalue_2 (`KismetMaterialLibrary.CreateDynamicMaterialInstance` "/Game/Drawing/M_Board.M_Board"))
      (`MaterialInstanceDynamic.SetTextureParameterValue` _returnvalue_2 "RenderTarget" (`self.RenderTarget`))
      (`PrimitiveComponent.SetMaterial` (`self.StaticMesh`) 0 _returnvalue_2))
    (:`then_2`
      ;[1 1 1] Loading brush material
      (bind _returnvalue_3 (`KismetMaterialLibrary.CreateDynamicMaterialInstance` "/Game/Drawing/M_Brush.M_Brush"))
      (set `self.BrushMaterial` _returnvalue_3))))

(event `self.HoldInteract`
  (params (HitResult :type "HitResult Structure (by ref)"))
  (bind _outhit (`KismetSystemLibrary.LineTraceSingle` :`Start` HitResult_TraceStart :`End` HitResult_TraceEnd :`TraceChannel` "TraceTypeQuery1" :`bTraceComplex` true :`DrawDebugType` "ForDuration"))
  (`KismetSystemLibrary.PrintString` "Hello")
  (`self.DrawBrush` "/Game/Drawing/Мел.Мел" 2.5 (`GameplayStatics.FindCollisionUV` _outhit)))

(fn `DrawBrush`
  (params (brushTexture :type "Texture2D Object Reference") (BrushSize :type "Float (double-precision)") (DrawLocation :type "Vector2D Structure"))
  (bind _brushsize (`local.BrushSize`))
  (`|ExecutionSequence`
    (:`then_0`
      ;[1 1 1] Choosing a texture to draw
      (`MaterialInstanceDynamic.SetTextureParameterValue` (`self.BrushMaterial`) "BrushTexture" brushTexture))
    (:`then_1`
      ;[1 1 1] Parameters for the brush
      (bind (_canvas _size _context) (`KismetRenderingLibrary.BeginDrawCanvasToRenderTarget` (`self.RenderTarget`)))
      (`Canvas.K2_DrawMaterial` _canvas (`self.BrushMaterial`) (- (* _size (`local.DrawLocation`)) (/ _brushsize 2.0)) (`KismetMathLibrary.MakeVector2D` _brushsize _brushsize) (0.0 0.0) (1.0 1.0) 0.0 (0.5 0.5))
      (`KismetRenderingLibrary.EndDrawCanvasToRenderTarget` _context))))

(fn `UserConstructionScript`)