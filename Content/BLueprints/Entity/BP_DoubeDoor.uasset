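; A proximity door actor that swings a single door mesh open near Pawns and shut when they are away, with sound.
; Each Tick loops over every Pawn, using FInterpTo to ease mesh yaw toward open or closed based on that Pawn's distance.
; Only the out-of-range branch triggers open and close sounds, using a near-zero yaw check, the DoorClosed flag and a DoOnce.
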(event `self.ReceiveBeginPlay`)

(event `self.ReceiveTick`
  (params (DeltaSeconds :type "Float (single-precision)"))
  (bind _audio (`self.Audio`))
  (bind _audio_2 (`self.Audio`))
  (bind (_relativerotation_roll _relativerotation_pitch _relativerotation_yaw) (`KismetMathLibrary.BreakRotator` (`SceneComponent.RelativeRotation` (`self.DoorMesh`))))
  (bind (_relativerotation_roll_2 _relativerotation_pitch_2 _relativerotation_yaw_2) (`KismetMathLibrary.BreakRotator` (`SceneComponent.RelativeRotation` (`self.DoorMesh`))))
  (bind _returnvalue (`KismetMathLibrary.FInterpTo` _relativerotation_yaw 0.0 (`GameplayStatics.GetWorldDeltaSeconds`) 2.0))
  (bind _outactors (`GameplayStatics.GetAllActorsOfClass` "/Script/Engine.Pawn"))
  (for _array_element _outactors
    (if (> (`self.GetDistanceTo` _array_element) 200.0)
      (`SceneComponent.K2_SetRelativeRotation` (`self.DoorMesh`) (`KismetMathLibrary.MakeRotator` 0.0 0.0 _returnvalue) false false)
      (if (`KismetMathLibrary.NearlyEqual_FloatFloat` _returnvalue 0.0 5.0)
        (if (`self.DoorClosed`)
          (`/Engine/EditorBlueprintResources/StandardMacros.DoOnce` true :!label _label
            (:`Completed`
              (`AudioComponent.SetSound` _audio_2 "/Game/Sounds/Door/SW_Door_Close.SW_Door_Close")
              (`AudioComponent.Play` _audio_2 0.0)
              (`KismetSystemLibrary.Delay` (`SoundBase.Duration` (`AudioComponent.Sound` _audio_2)))
              (`AudioComponent.Stop` _audio_2))))
        (set `self.DoorClosed` false)
        (else
          (if (not (`self.DoorClosed`))
            (`AudioComponent.SetSound` _audio "/Game/Sounds/Door/SW_Door_Open.SW_Door_Open")
            (`AudioComponent.Play` _audio 0.0)
            (`KismetSystemLibrary.Delay` (`SoundBase.Duration` (`AudioComponent.Sound` _audio)))
            (`AudioComponent.Stop` _audio))
          (set `self.DoorClosed` true)
          (goto _label :!via `Reset`)))
      (else
        (`SceneComponent.K2_SetRelativeRotation` (`self.DoorMesh`) (`KismetMathLibrary.MakeRotator` 0.0 0.0 (`KismetMathLibrary.FInterpTo` _relativerotation_yaw_2 250.0 (`GameplayStatics.GetWorldDeltaSeconds`) 2.0)) false false)))))

(fn `UserConstructionScript`)