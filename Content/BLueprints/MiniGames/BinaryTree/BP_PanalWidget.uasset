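; BP_PanalWidget is the in-world panel of the BinaryTree minigame, showing a button widget and timing how long the interaction lasts.
; When the random-work-start event fires, it puts BPW_PanalButtonsWidget in the widget component, requests randomized images and starts a looping one-second Delay counter for minutes and seconds.
; EndInteract clears EndTimer, which stops the loop and prints the time, then swaps in BPW_None and resets the answer text.
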(event `self.ReceiveBeginPlay`
  ;[0 0 0] Random images and start timer
  (add `self.RandomWorkStart` (delegate `Random`)))

(event `Random`
  ;[0 0 0] Random images and start timer
  (set `self.EndTimer` true)
  (add `self.StartTimer` (delegate `Timer`))
  (`self.StartTimer`)
  (bind _returnvalue (`|CreateWidget` "/Game/BLueprints/MiniGames/BinaryTree/BPW_PanalButtonsWidget.BPW_PanalButtonsWidget_C"))
  (`WidgetComponent.SetWidget` (`self.WidgetComponent`) _returnvalue)
  (message `/Game/BLueprints/MiniGames/BinaryTree/BPI_InterfaceRandomInteraction.RandomImages` _returnvalue))

(event `Timer`
  ;[0 0 0] Timer
  (`KismetSystemLibrary.Delay` 1.0 :!label _label)
  (bind _output_get (set `self.Seconds` (+ (`self.Seconds`) 1)))
  (if (== _output_get 60)
    (set `self.Seconds` 0)
    (set `self.Minuts` (+ (`self.Minuts`) 1)))
  (if (`self.EndTimer`)
    (goto _label)
    (else
      (`KismetSystemLibrary.PrintString` (`KismetStringLibrary.Conv_IntToString` (`self.Seconds`)))
      (`KismetSystemLibrary.PrintString` (`KismetStringLibrary.Conv_IntToString` (`self.Minuts`))))))

(event `self.EndInteract`
  ;[0 0 0] End Interact and End timer
  (set `self.EndTimer` false)
  (bind _returnvalue (`|CreateWidget` "/Game/BLueprints/MiniGames/BinaryTree/BPW_None.BPW_None_C"))
  (`WidgetComponent.SetWidget` (`self.WidgetComponent`) _returnvalue)
  (`TextRenderComponent.K2_SetText` (`self.Answerss`) (`self.NoneText`)))

(fn `UserConstructionScript`)