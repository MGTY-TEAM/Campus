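; Camera pawn for the chess minigame that provides mouse-driven look and zoom.
; Holding the right mouse button opens a gate on Tick that feeds mouse movement into controller yaw and inverted pitch.
; The mouse wheel changes the spring arm length in small clamped steps, with wheel up lengthening the arm and wheel down shortening it.
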(event `Key|RightMouseButton`
  (params (Key :type "Key Structure"))
  (:`Pressed`
    (goto _label :!via `Open`))
  (:`Released`
    (goto _label :!via `Close`)))

(event `self.ReceiveTick`
  (params (DeltaSeconds :type "Float (single-precision)"))
  (`/Engine/EditorBlueprintResources/StandardMacros.Gate` true :!label _label
    (:`Exit`
      (`|ExecutionSequence`
        (:`then_0`
          (`self.AddControllerYawInput` (`self.GetInputAxisValue`)))
        (:`then_1`
          (`self.AddControllerPitchInput` (* (`self.GetInputAxisValue`) -1.0)))))))

(event `self.ReceiveBeginPlay`)

(event `Key|MouseScrollUp`
  (params (Key :type "Key Structure"))
  (bind _springarmcomponent (`self.SpringArmComponent`))
  (:`Pressed`
    (set `SpringArmComponent.TargetArmLength` (`KismetMathLibrary.FClamp` (+ (`SpringArmComponent.TargetArmLength` _springarmcomponent) 2.0) 40.0 70.0) _springarmcomponent)))

(event `Key|MouseScrollDown`
  (params (Key :type "Key Structure"))
  (bind _springarmcomponent (`self.SpringArmComponent`))
  (:`Pressed`
    (set `SpringArmComponent.TargetArmLength` (`KismetMathLibrary.FClamp` (+ (`SpringArmComponent.TargetArmLength` _springarmcomponent) -2.0) 40.0 70.0) _springarmcomponent)))

(fn `UserConstructionScript`)