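; Space object with rings for the Solar System minigame, handling how the planet resets to its begin position.
; ReallocatePlanet creates a dynamic material on the mesh's first slot at zero opacity, moves the actor back and re-enables pickup.
; A timeline's DissolveTrack then drives the Opacity parameter so the object fades at its restored position rather than popping in.
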(event `self.ReallocatePlanet`
  (`|ExecutionSequence`
    (:`then_0`
      (`/Engine/EditorBlueprintResources/StandardMacros.IsValid` (`self.StaticMeshComponent`)
        (:`Is Valid`
          (`/Engine/EditorBlueprintResources/StandardMacros.IsValid` (`PrimitiveComponent.GetMaterial` (`self.StaticMeshComponent`) 0)
            (:`Is Valid`
              (bind _returnvalue (`PrimitiveComponent.CreateDynamicMaterialInstance` (`self.StaticMeshComponent`) 0 (`PrimitiveComponent.GetMaterial` (`self.StaticMeshComponent`) 0) "None"))
              (bind _output_get (set `self.Dyn_Material` _returnvalue))
              (`/Engine/EditorBlueprintResources/StandardMacros.IsValid` _output_get
                (:`Is Valid`
                  (`MaterialInstanceDynamic.SetScalarParameterValue` (`self.Dyn_Material`) "Opacity" 0.0)
                  (`PrimitiveComponent.SetMaterial` (`self.StaticMeshComponent`) 0 (`self.Dyn_Material`)))))))))
    (:`then_1`
      (`self.K2_SetActorLocation` (`self.GetBeginPosition`))
      (`self.SetCanPickup` true))
    (:`then_2`
      (bind (_direction _dissolvetrack) (`Timeline|Timeline` :!via `PlayFromStart`)
        (:`Update`
          (`/Engine/EditorBlueprintResources/StandardMacros.IsValid` (`self.StaticMeshComponent`)
            (:`Is Valid`
              (`MaterialInstanceDynamic.SetScalarParameterValue` (`self.Dyn_Material`) "Opacity" _dissolvetrack))))))))

(fn `UserConstructionScript`)