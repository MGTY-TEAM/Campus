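; BP_SpaceObject is a pickupable object in the SolarSystem minigame that can be reset to its begin position with a fade-in.
; ReallocatePlanet creates a dynamic material for the mesh's first slot, zeroes its opacity, then moves the actor back and re-enables pickup.
; A timeline's dissolve track then drives the Opacity parameter to reveal the planet.
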(event `self.ReallocatePlanet`
  (bind _staticmeshcomponent (`self.StaticMeshComponent`))
  (bind _returnvalue (`PrimitiveComponent.GetMaterial` _staticmeshcomponent 0))
  (`|ExecutionSequence`
    (:`then_0`
      (`/Engine/EditorBlueprintResources/StandardMacros.IsValid` _staticmeshcomponent
        (:`Is Valid`
          (`/Engine/EditorBlueprintResources/StandardMacros.IsValid` _returnvalue
            (:`Is Valid`
              (bind _returnvalue_2 (`PrimitiveComponent.CreateDynamicMaterialInstance` (`self.StaticMeshComponent`) 0 _returnvalue "None"))
              (bind _output_get (set `self.Dyn_Material` _returnvalue_2))
              (`/Engine/EditorBlueprintResources/StandardMacros.IsValid` _output_get
                (:`Is Valid`
                  (`MaterialInstanceDynamic.SetScalarParameterValue` (`self.Dyn_Material`) "Opacity" 0.0)
                  (`PrimitiveComponent.SetMaterial` (`self.StaticMeshComponent`) 0 (`self.Dyn_Material`)))))))))
    (:`then_1`
      (`self.K2_SetActorLocation` (`self.GetBeginPosition`))
      (`self.SetCanPickup` true))
    (:`then_2`
      (bind (_direction _dissolvetrack) (`Timeline|Timeline` :!via `PlayFromStart`)
        (:`Update`
          (`/Engine/EditorBlueprintResources/StandardMacros.IsValid` (`self.StaticMeshComponent`)
            (:`Is Valid`
              (`MaterialInstanceDynamic.SetScalarParameterValue` (`self.Dyn_Material`) "Opacity" _dissolvetrack))))))))

(fn `UserConstructionScript`)