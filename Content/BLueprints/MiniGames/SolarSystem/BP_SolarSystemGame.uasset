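; BP_SolarSystemGame is the solar system minigame Blueprint, which here only handles the lighting change when the game is completed.
; On OnGameCompleted it loops through LampsToOff, casts each entry to BP_Lamp, swaps a mesh material to M_Lamp_0 and sets the RectLight intensity to zero.
; It has no other active logic in its event graph or construction script.
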(event `self.OnGameCompleted`
  (if (> (`KismetArrayLibrary.Array_Length` (`self.LampsToOff`)) 0)
    (for _array_element (`self.LampsToOff`)
      (bind _asbp_lamp (cast `/Game/Mesh/BlueprintsProjectSchool/BP_Lamp` _array_element))
      (`PrimitiveComponent.SetMaterial` (`/Game/Mesh/BlueprintsProjectSchool/BP_Lamp.StaticMesh` _asbp_lamp) 1 "/Game/Materials/ProjectSchool/Lamp/M_Lamp_0.M_Lamp_0")
      (`LightComponent.SetIntensity` (`/Game/Mesh/BlueprintsProjectSchool/BP_Lamp.RectLight` _asbp_lamp) 0.0))))

(event `self.ReceiveBeginPlay`)

(fn `UserConstructionScript`)