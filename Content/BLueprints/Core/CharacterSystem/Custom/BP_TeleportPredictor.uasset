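; BP_TeleportPredictor is an actor that previews a teleport arc and landing point, storing the target location and its validity.
; While prediction runs through a Tick-fed gate, it traces a projectile path from the Arrow, ignoring the player pawn.
; Hits update the spline and Niagara trail, then project the endpoint onto navigation to place the marker.
; Prediction starts and stops via events, auto-starting on BeginPlay when ownerless.
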(event `self.ReceiveBeginPlay`
  (if (not (`KismetSystemLibrary.IsValid` (`self.GetOwner`)))
    (`self.StartPredict`)))

(event `StartPredict`
  (bind _arrow (`self.Arrow`))
  (goto _label :!via `Open`))

(event `StopPredict`
  (bind _arrow (`self.Arrow`))
  (goto _label :!via `Close`))

(event `self.ReceiveTick`
  (params (DeltaSeconds :type "Float (single-precision)"))
  (bind _arrow (`self.Arrow`))
  (`/Engine/EditorBlueprintResources/StandardMacros.Gate` true :!label _label
    (:`Exit`
      (bind (_outhit _outpathpositions _outlasttracedestination _returnvalue) (`GameplayStatics.Blueprint_PredictProjectilePath_ByTraceChannel` (`SceneComponent.K2_GetComponentLocation` _arrow) (* (`SceneComponent.GetForwardVector` _arrow) (`self.Force`)) true 10.0 "ECC_WorldStatic" false (`|MakeArray` (`GameplayStatics.GetPlayerPawn` 0) :!type "Actor Object Reference")))
      (if _returnvalue
        (`SplineComponent.SetSplinePoints` (`self.Spline`) _outpathpositions "World" true)
        (`NiagaraDataInterfaceArrayFunctionLibrary.SetNiagaraArrayVector` (`self.NS_TeleportTrace`) "User.PointArray" _outpathpositions)
        (bind (_projectedlocation _returnvalue_2) (`NavigationSystemV1.K2_ProjectPointToNavigation` _outlasttracedestination))
        (`SceneComponent.K2_SetWorldLocation` (`self.FinalPoint`) _projectedlocation false false)
        (`SceneComponent.K2_SetWorldRotation` :`self` (`self.FinalPoint`))
        (set `self.LastLocationIsValid` _returnvalue_2)
        (set `self.TeleportLocation` _projectedlocation)))))

(fn `UserConstructionScript`)