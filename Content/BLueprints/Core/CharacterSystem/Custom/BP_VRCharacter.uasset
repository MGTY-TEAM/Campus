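; BP_VRCharacter is the player's VR character, adding the IMC_VR Enhanced Input context on BeginPlay and handling teleport, UI clicks and a menu.
; Holding IA_Move runs a child-actor BP_TeleportPredictor; release moves the character to its valid target in X and Y, keeping current Z.
; Per-hand inputs click through two WidgetInteraction components, and the menu input toggles the Widget component's visibility.
; IA_VR_ProcessInteraction forwards axis values to left and right hand events, which are empty here.
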(event `self.ReceiveBeginPlay`
  (bind _asplayer_controller (cast `PlayerController` (`self.GetController`)))
  (`EnhancedInputSubsystemInterface.AddMappingContext` (pcsubsystem `EnhancedInputLocalPlayerSubsystem` _asplayer_controller) "/Game/BLueprints/Core/CharacterSystem/Input/Action/VR/IMC_VR.IMC_VR" 0 (struct))
  (bind _asbp_teleport_predictor (cast `/Game/BLueprints/Core/CharacterSystem/Custom/BP_TeleportPredictor` (`ChildActorComponent.ChildActor` (`self.TeleportPredictor`))))
  (set `self.TeleportVisualiser` _asbp_teleport_predictor))

(event `EnhancedInput|/Game/BLueprints/Core/CharacterSystem/Input/Action/IA_Move`
  (params (ActionValue :type "Vector2D Structure") (ElapsedSeconds :type "Float (double-precision)") (TriggeredSeconds :type "Float (double-precision)") (InputAction :type "InputAction Object Reference" :default "/Game/BLueprints/Core/CharacterSystem/Input/Action/IA_Move.IA_Move"))
  (bind (_returnvalue_x _returnvalue_y _returnvalue_z) (`KismetMathLibrary.BreakVector` (`self.K2_GetActorLocation`)))
  (bind _teleportvisualiser (`self.TeleportVisualiser`))
  (bind _teleportvisualiser_2 (`self.TeleportVisualiser`))
  (bind (_teleportlocation_x _teleportlocation_y) (`KismetMathLibrary.BreakVector` (`/Game/BLueprints/Core/CharacterSystem/Custom/BP_TeleportPredictor.TeleportLocation` _teleportvisualiser)))
  (:`Started`
    (`SceneComponent.SetVisibility` (`self.TeleportPredictor`) true false)
    (if (`KismetSystemLibrary.IsValid` _teleportvisualiser_2)
      (`/Game/BLueprints/Core/CharacterSystem/Custom/BP_TeleportPredictor.StartPredict` _teleportvisualiser_2)))
  (:`Completed`
    (`SceneComponent.SetVisibility` (`self.TeleportPredictor`) false false)
    (if (`KismetSystemLibrary.IsValid` _teleportvisualiser)
      (`/Game/BLueprints/Core/CharacterSystem/Custom/BP_TeleportPredictor.StopPredict` _teleportvisualiser)
      (if (`/Game/BLueprints/Core/CharacterSystem/Custom/BP_TeleportPredictor.LastLocationIsValid` _teleportvisualiser)
        (`self.K2_SetActorLocation` (`KismetMathLibrary.MakeVector` _teleportlocation_x _teleportlocation_y _returnvalue_z))))))

(event `EnhancedInput|/Game/BLueprints/Core/CharacterSystem/Input/Action/VR/IA_VR_ProcessInteraction`
  (params (ActionValue :type "Vector2D Structure") (ElapsedSeconds :type "Float (double-precision)") (TriggeredSeconds :type "Float (double-precision)") (InputAction :type "InputAction Object Reference" :default "/Game/BLueprints/Core/CharacterSystem/Input/Action/VR/IA_VR_ProcessInteraction.IA_VR_ProcessInteraction"))
  (:`Triggered`
    (`self.RightHandInteraction` ActionValue_X)
    (`self.LeftHandInteraction` ActionValue_Y)))

(event `RightHandInteraction`
  (params (Input :type "Float (double-precision)")))

(event `EnhancedInput|/Game/BLueprints/Core/CharacterSystem/Input/Action/VR/IA_VR_RightHandInteraction`
  (params (ActionValue :type Boolean) (ElapsedSeconds :type "Float (double-precision)") (TriggeredSeconds :type "Float (double-precision)") (InputAction :type "InputAction Object Reference" :default "/Game/BLueprints/Core/CharacterSystem/Input/Action/VR/IA_VR_RightHandInteraction.IA_VR_RightHandInteraction"))
  (bind _widgetinteraction (`self.WidgetInteraction`))
  (:`Triggered`
    (`WidgetInteractionComponent.PressPointerKey` _widgetinteraction "LeftMouseButton")
    (`WidgetInteractionComponent.ReleasePointerKey` _widgetinteraction "LeftMouseButton")))

(event `LeftHandInteraction`
  (params (Input :type "Float (double-precision)")))

(event `EnhancedInput|/Game/BLueprints/Core/CharacterSystem/Input/Action/VR/IA_VR_LeftHand_Interaction`
  (params (ActionValue :type Boolean) (ElapsedSeconds :type "Float (double-precision)") (TriggeredSeconds :type "Float (double-precision)") (InputAction :type "InputAction Object Reference" :default "/Game/BLueprints/Core/CharacterSystem/Input/Action/VR/IA_VR_LeftHand_Interaction.IA_VR_LeftHand_Interaction"))
  (bind _widgetinteraction1 (`self.WidgetInteraction1`))
  (:`Triggered`
    (`WidgetInteractionComponent.PressPointerKey` _widgetinteraction1 "LeftMouseButton")
    (`WidgetInteractionComponent.ReleasePointerKey` _widgetinteraction1 "LeftMouseButton")))

(event `EnhancedInput|/Game/BLueprints/Core/CharacterSystem/Input/Action/VR/IA_VR_OpenMenu`
  (params (ActionValue :type Boolean) (ElapsedSeconds :type "Float (double-precision)") (TriggeredSeconds :type "Float (double-precision)") (InputAction :type "InputAction Object Reference" :default "/Game/BLueprints/Core/CharacterSystem/Input/Action/VR/IA_VR_OpenMenu.IA_VR_OpenMenu"))
  (:`Triggered`
    (`/Engine/EditorBlueprintResources/StandardMacros.FlipFlop`
      (:`A`
        (`SceneComponent.SetVisibility` (`self.Widget`) true false))
      (:`B`
        (`SceneComponent.SetVisibility` (`self.Widget`) false false)))))

(fn `UserConstructionScript`)