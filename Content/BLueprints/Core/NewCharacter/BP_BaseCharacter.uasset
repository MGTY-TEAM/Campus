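; Base character Blueprint that drives camera autofocus for depth of field, despite its function being named Calculate FOV.
; Each Tick, it line traces on Visibility along the camera's forward vector to measure the distance to the surface in view.
; On a hit, it rebuilds the camera's post-process settings with fixed aperture and exposure values, easing focal distance toward that point with FInterpTo.
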(event `self.ReceiveTick`
  (params (DeltaSeconds :type "Float (single-precision)"))
  (`self.Calculate FOV` 2.5 5.0 11.0 1.0))

(event `self.ReceiveBeginPlay`)

(fn `Calculate FOV`
  (params (InterpSpeed :type "Float (double-precision)") (`Exposure Compensation` :type "Float (single-precision)") (`Maximum Aperture (min F-stop)` :type "Float (single-precision)") (`Aperture (F-stop)` :type "Float (single-precision)"))
  (bind _cameracomponent (`self.CameraComponent`))
  (bind _cameracomponent_2 (`self.CameraComponent`))
  (bind _returnvalue (`SceneComponent.K2_GetComponentLocation` _cameracomponent_2))
  (bind (_outhit _returnvalue_2) (`KismetSystemLibrary.LineTraceSingle` _returnvalue (+ _returnvalue (* (`SceneComponent.GetForwardVector` _cameracomponent_2) 10000)) "TraceTypeQuery1"))
  (if _returnvalue_2
    (bind _output_get (set `self.Focus Distance` (`KismetMathLibrary.VSize` (- (`.Location` (`GameplayStatics.BreakHitResult` _outhit)) (`SceneComponent.K2_GetComponentLocation` (`self.CameraComponent`))))))
    (set `CameraComponent.PostProcessSettings` (make `PostProcessSettings` :`DepthOfFieldFstop` `Aperture (F-stop)` :`DepthOfFieldMinFstop` `Maximum Aperture (min F-stop)` :`AutoExposureBias` `Exposure Compensation` :`DepthOfFieldFocalDistance` (`KismetMathLibrary.FInterpTo` (`.DepthOfFieldFocalDistance` (break `PostProcessSettings` (`CameraComponent.PostProcessSettings` _cameracomponent))) _output_get (`GameplayStatics.GetWorldDeltaSeconds`) InterpSpeed)) _cameracomponent)))

(fn `UserConstructionScript`)