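; Interactive blackboard that the player draws on with chalk by holding interact.
; A line trace's hit UV places a brush material on a runtime render target, which a dynamic material shows on all three board meshes.
; The chalk mesh eases after the impact point while ChalkMove plays.
; A retriggerable delay opens a Tick gate after drawing pauses, easing the chalk home, stopping ChalkMove and playing a return sound.
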(event `self.ReceiveBeginPlay`
  (set `self.Init Coord` (`SceneComponent.K2_GetComponentLocation` (`self.Chalk`)))
  (`|ExecutionSequence`
    (:`then_0`
      ;[1 1 1] Creating a drawing area
      (bind _returnvalue (`KismetRenderingLibrary.CreateRenderTarget2D` 2048 2048))
      (bind _output_get (set `self.RenderTarget` _returnvalue))
      (`KismetRenderingLibrary.DrawMaterialToRenderTarget` _output_get "/Game/Materials/BlackboardDrawing/M_Board.M_Board"))
    (:`then_1`
      ;[1 1 1] Loading the board material
      (bind _returnvalue_2 (`KismetMaterialLibrary.CreateDynamicMaterialInstance` "/Game/Materials/BlackboardDrawing/M_Board.M_Board"))
      (`MaterialInstanceDynamic.SetTextureParameterValue` _returnvalue_2 "RenderTarget" (`self.RenderTarget`))
      (`PrimitiveComponent.SetMaterial` (`self.Board_Main`) 0 _returnvalue_2)
      (`PrimitiveComponent.SetMaterial` (`self.Board_Left`) 0 _returnvalue_2)
      (`PrimitiveComponent.SetMaterial` (`self.Board_Right`) 0 _returnvalue_2))
    (:`then_2`
      ;[1 1 1] Loading brush material
      (bind _returnvalue_3 (`KismetMaterialLibrary.CreateDynamicMaterialInstance` "/Game/Materials/BlackboardDrawing/M_Brush.M_Brush"))
      (set `self.BrushMaterial` _returnvalue_3))))

(event `self.ReceiveTick`
  (params (DeltaSeconds :type "Float (single-precision)"))
  ;[1 1 1] Moving the chalk component to the initial coordinates
  (`/Engine/EditorBlueprintResources/StandardMacros.Gate` true :!label _label
    (:`Exit`
      (`self.ReturnChalk` (`SceneComponent.K2_GetComponentLocation` (`self.Chalk`)))
      ;[1 1 1] Return Chalk Sound
      (if (and (== (`KismetMathLibrary.Conv_DoubleToInt64` (.y (`SceneComponent.K2_GetComponentLocation` (`self.Chalk`)))) (`KismetMathLibrary.Conv_DoubleToInt64` (.y (`self.Init Coord`)))) (== (`KismetMathLibrary.Conv_DoubleToInt64` (.z (`SceneComponent.K2_GetComponentLocation` (`self.Chalk`)))) (`KismetMathLibrary.Conv_DoubleToInt64` (.z (`self.Init Coord`)))))
        (`/Engine/EditorBlueprintResources/StandardMacros.DoOnce` false :!label _label_2
          (:`Completed`
            (`KismetSystemLibrary.Delay` 0.5)
            (`GameplayStatics.PlaySound2D` "/Game/Sounds/Chalk/SW_Chalk_Return.SW_Chalk_Return" 0.4 1.0 0.0 null null)))
        (else
          (goto _label_2 :!via `Reset`))))))

(event `self.HoldInteract`
  (params (HitResult :type "HitResult Structure (by ref)"))
  ;[1 1 1] Drawing a chalk texture on a blackboard
  (bind _outhit (`KismetSystemLibrary.LineTraceSingle` :`Start` HitResult_TraceStart :`End` HitResult_TraceEnd :`TraceChannel` "TraceTypeQuery1" :`bTraceComplex` true :`bIgnoreSelf` false))
  (`self.DrawBrush` "/Game/Textures/BlackboardDrawing/T_Chalk.T_Chalk" 3.0 (`GameplayStatics.FindCollisionUV` _outhit))
  ;[1 1 1] Movement of the chalk component on the board
  (`self.ChalkAnimation` (`.ImpactPoint` (`GameplayStatics.BreakHitResult` _outhit)))
  ;[1 1 1] Moving the chalk component to the initial coordinates
  (`KismetSystemLibrary.RetriggerableDelay` 0.5)
  (goto _label :!via `Open`))

(event `self.BPInteract`
  (params (HitResult :type "HitResult Structure (by ref)"))
  ;[1 1 1] Moving the chalk component to the initial coordinates
  (`AudioComponent.Play` (`self.Chalk_Move`) 0.0)
  (goto _label :!via `Close`))

(fn `CanInteract`
  (returns (ReturnValue :type Boolean))
  (return false))

(fn `ChalkAnimation`
  (params (`Impact Point` :type "Vector Structure"))
  (locals (NewLocalVar :type "Float (double-precision)" :default 0.0))
  (bind _returnvalue (`GameplayStatics.GetWorldDeltaSeconds`))
  (`SceneComponent.K2_SetWorldTransform` (`self.Chalk`) (`KismetMathLibrary.MakeTransform` (`KismetMathLibrary.MakeVector` (+ (.x `Impact Point`) 2.0) (`KismetMathLibrary.FInterpTo` (.y (`SceneComponent.K2_GetComponentLocation` (`self.Chalk`))) (.y `Impact Point`) _returnvalue 11.0) (`KismetMathLibrary.FInterpTo` (.z (`SceneComponent.K2_GetComponentLocation` (`self.Chalk`))) (.z `Impact Point`) _returnvalue 11.0)) (struct :`Pitch` -20.0) (`SceneComponent.K2_GetComponentScale` (`self.Chalk`))) false false))

(fn `DrawBrush`
  (params (brushTexture :type "Texture2D Object Reference") (BrushSize :type "Float (double-precision)") (DrawLocation :type "Vector2D Structure"))
  (bind _brushsize (`local.BrushSize`))
  (`|ExecutionSequence`
    (:`then_0`
      ;[1 1 1] Choosing a texture to draw
      (`MaterialInstanceDynamic.SetTextureParameterValue` (`self.BrushMaterial`) "BrushTexture" brushTexture))
    (:`then_1`
      ;[1 1 1] Parameters for the brush
      (bind (_canvas _size _context) (`KismetRenderingLibrary.BeginDrawCanvasToRenderTarget` (`self.RenderTarget`)))
      (`Canvas.K2_DrawMaterial` _canvas (`self.BrushMaterial`) (- (* _size (`local.DrawLocation`)) (/ _brushsize 2.0)) (`KismetMathLibrary.MakeVector2D` _brushsize _brushsize) (0.0 0.0) (1.0 1.0) 0.0 (0.5 0.5))
      (`KismetRenderingLibrary.EndDrawCanvasToRenderTarget` _context))))

(fn `ReturnChalk`
  (params (`Chalk Location` :type "Vector Structure"))
  (bind _returnvalue (`GameplayStatics.GetWorldDeltaSeconds`))
  (bind (_returnvalue_roll _returnvalue_pitch _returnvalue_yaw) (`KismetMathLibrary.BreakRotator` (`SceneComponent.K2_GetComponentRotation` (`self.Chalk`))))
  (`SceneComponent.K2_SetWorldTransform` (`self.Chalk`) (`KismetMathLibrary.MakeTransform` (`KismetMathLibrary.MakeVector` (.x `Chalk Location`) (`KismetMathLibrary.FInterpTo` (.y `Chalk Location`) (.y (`self.Init Coord`)) _returnvalue 3.0) (`KismetMathLibrary.FInterpTo` (.z `Chalk Location`) (.z (`self.Init Coord`)) _returnvalue 3.0)) (`KismetMathLibrary.MakeRotator` 0.0 0.0 (`KismetMathLibrary.FInterpTo` _returnvalue_yaw 90.0 _returnvalue 3.0)) (`SceneComponent.K2_GetComponentScale` (`self.Chalk`))) false false)
  (`AudioComponent.Stop` (`self.Chalk_Move`)))

(fn `UserConstructionScript`)