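; BP_DraggedActor is an interactable physics object that is dragged horizontally toward where the interaction trace points.
; DragInteract intersects the trace from its HitResult with a horizontal plane at the actor's location.
; It applies a force to the Cube toward that point, scaled by Strength and clamped offset distance, so the pull levels off when far away.
; A leftover debug "Hello" prints on every call.
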(event `self.DragInteract`
  (params (HitResult :type "HitResult Structure (by ref)"))
  (bind (_t _intersection _returnvalue) (`KismetMathLibrary.LinePlaneIntersection` HitResult_TraceStart HitResult_TraceEnd (`KismetMathLibrary.MakePlaneFromPointAndNormal` (`self.K2_GetActorLocation`) (0.0 0.0 1.0))))
  ;[1 1 1] Get Interaction vector and Validate
  (`KismetSystemLibrary.PrintString` "Hello")
  (if (> (`KismetMathLibrary.VSize` (- HitResult_TraceEnd HitResult_TraceStart)) 0.0)
    (if _returnvalue
      ;[1 1 1] Add Drag Force
      (`PrimitiveComponent.AddForce` (`self.Cube`) (* (`self.Strength`) (`KismetMathLibrary.ClampVectorSize` (- _intersection (`self.K2_GetActorLocation`)) 0.0 100.0)) "None" false))))

(fn `UserConstructionScript`)